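; Medium enemy AI that turns to face the player and shoots when within attack range.
; Each Tick updates the range flag from player distance, then runs rotation and firing.
; The capsule interpolates toward the player's look-at rotation, with pitch offset by barrel length and clamped.
; A Delay on the Tick-driven fire path paces projectile spawns from the capsule socket, each triggering particles and a 2D shot sound.
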(event `self.ReceiveTick`
  (params (DeltaSeconds :type "Float (single-precision)"))
  ;[1 1 1] GameLoop
  (set `self.DeltaTime` DeltaSeconds)
  (`self.UpdateRange`)
  (`self.UpdateRotation`)
  (`self.FireWaepons`))

(event `UpdateRotation`
  ;[1 1 1] SeguirPersonagem
  (if (`self.EnemyInRange`)
    (`SceneComponent.K2_SetWorldRotation` (`self.CapsuleComponent`) (`KismetMathLibrary.RInterpTo` (`SceneComponent.K2_GetComponentRotation` (`self.CapsuleComponent`)) (`KismetMathLibrary.MakeRotator` 0.0 (`KismetMathLibrary.ClampAngle` (- (.pitch (`KismetMathLibrary.FindLookAtRotation` (`SceneComponent.K2_GetComponentLocation` (`self.CapsuleComponent`)) (`self.K2_GetActorLocation` (`GameplayStatics.GetPlayerPawn` 0)))) (`self.BarrelLeght`)) -10.0 35.0) (.yaw (`KismetMathLibrary.FindLookAtRotation` (`SceneComponent.K2_GetComponentLocation` (`self.CapsuleComponent`)) (`self.K2_GetActorLocation` (`GameplayStatics.GetPlayerPawn` 0))))) (`self.DeltaTime`) (`self.RotationSpeed`)) false false)))

(event `FireWaepons`
  ;[1 1 1] Atirar
  (if (`self.EnemyInRange`)
    (`KismetSystemLibrary.Delay` (`self.Fire`))
    (bind _returnvalue (`|SpawnActorFromClass` "/Script/Jogo.ProjectileActor" (`SceneComponent.GetSocketTransform` (`self.CapsuleComponent`) "Socket" "RTS_World") "Undefined" "OverrideRootScale"))
    (`ProjectileActor.Particulas` _returnvalue 2)
    (`GameplayStatics.PlaySound2D` "/Game/Sounds/Inimigos/RobotShoot.RobotShoot")))

(event `UpdateRange`
  ;[1 1 1] Range
  (if (<= (`self.GetDistanceTo` self (`GameplayStatics.GetPlayerPawn` 0)) (`self.AtackRange`))
    (set `self.EnemyInRange` true)
    (else
      (set `self.EnemyInRange` false))))

(fn `UserConstructionScript`)